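; Base item actor that represents either an item or a weapon in the world and destroys itself when its trigger overlaps a component tagged EventSuccess.
; On BeginPlay, a "Random" DataType resolves evenly to Item or Weapon, with a row number rolled within that type's configured range.
; GetData then reads that row from the matching data table, stores it in ItemData, and applies its mesh with a type-specific transform.
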(event `self.ReceiveBeginPlay`
  (if (!= (`self.DataType`) "Random")
    _
    (elif (<= (`KismetMathLibrary.RandomIntegerInRange` 1 100) 50)
      (set `self.DataType` "Item")
      (set `self.ItemRowNum` (`KismetStringLibrary.Conv_StringToName` (`KismetStringLibrary.Conv_IntToString` (`KismetMathLibrary.RandomIntegerInRange` (`self.RandomMinItem`) (`self.RandomMaxItem`)))))
      (else
        (set `self.DataType` "Weapon")
        (set `self.ItemRowNum` (`KismetStringLibrary.Conv_StringToName` (`KismetStringLibrary.Conv_IntToString` (`KismetMathLibrary.RandomIntegerInRange` (`self.RandomMinWeapon`) (`self.RandomMaxWeapon`))))))))
  (`self.GetData`))

(event `self.GetTrigger.OnComponentBeginOverlap`
  (params (OverlappedComponent :type "PrimitiveComponent Object Reference") (OtherActor :type "Actor Object Reference") (OtherComp :type "PrimitiveComponent Object Reference") (OtherBodyIndex :type Integer) (bFromSweep :type Boolean) (SweepResult :type "HitResult Structure (by ref)"))
  (if (`ActorComponent.ComponentHasTag` OtherComp "EventSuccess")
    (`self.K2_DestroyActor`)))

(fn `GetData`
  (bind _datatype (`self.DataType`))
  (if (== _datatype "Item")
    (bind _returnvalue (`|GetDataTableRow` "/Game/DevelopTest/BluePrints/Item/DT_ItemData.DT_ItemData" (`self.ItemRowNum`))
      (:`then`
        (bind _output_get (set `self.ItemData` _returnvalue))
        (`StaticMeshComponent.SetStaticMesh` (`self.StaticMesh`) (`.Mesh_27_1F78B86F489209CDE44290B93B0038B2` (break `/Game/DevelopTest/BluePrints/Item/ST_ItemBase` _output_get)))
        (`SceneComponent.K2_SetRelativeTransform` (`self.StaticMesh`) (`KismetMathLibrary.MakeTransform` (0.0 0.0 0.0) (struct) (3.0 3.0 3.0)) false false)))
    (elif (== _datatype "Weapon")
      (bind _returnvalue_2 (`|GetDataTableRow` "/Game/DevelopTest/BluePrints/Item/DT_WeaponData.DT_WeaponData" (`self.ItemRowNum`))
        (:`then`
          (bind _output_get_2 (set `self.ItemData` _returnvalue_2))
          (`StaticMeshComponent.SetStaticMesh` (`self.StaticMesh`) (`.Mesh_27_1F78B86F489209CDE44290B93B0038B2` (break `/Game/DevelopTest/BluePrints/Item/ST_ItemBase` _output_get_2)))
          (`SceneComponent.K2_SetRelativeTransform` (`self.StaticMesh`) (`KismetMathLibrary.MakeTransform` (0.0 0.0 90.0) (struct :`Pitch` 180.0)) false false))))))

(fn `UserConstructionScript`)