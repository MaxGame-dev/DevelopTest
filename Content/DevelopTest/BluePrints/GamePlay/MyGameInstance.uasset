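; Game instance for a two-player LAN multiplayer test that handles sessions, level travel and stored player data.
; CreateSession opens TestLevel as a listen server, while JoinSession finds and joins the first LAN result, printing success or failure.
; MoveLevel opens a named level with the listen option, and SetPlayerData stores player data with a saved flag.
; Network and travel error handlers only print the failure type.
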(event `self.HandleNetworkError`
  (params (FailureType :type "ENetworkFailure Enum" :default "NetDriverAlreadyExists") (bIsServer :type Boolean))
  (switch `ENetworkFailure` FailureType
    (:`NetDriverAlreadyExists`
      _)
    (:`NetDriverCreateFailure`
      _)
    (:`NetDriverListenFailure`
      _)
    (:`ConnectionLost`
      _)
    (:`ConnectionTimeout`
      _)
    (:`FailureReceived`
      _)
    (:`OutdatedClient`
      _)
    (:`OutdatedServer`
      _)
    (:`PendingConnectionFailure`
      _)
    (:`NetGuidMismatch`
      _)
    (:`NetChecksumMismatch`
      _))
  (`KismetSystemLibrary.PrintString` (`|GetEnumeratorNameAsString` FailureType)))

(event `self.HandleTravelError`
  (params (FailureType :type "ETravelFailure Enum" :default "NoLevel"))
  (switch `ETravelFailure` FailureType
    (:`NoLevel`
      _)
    (:`LoadMapFailure`
      _)
    (:`InvalidURL`
      _)
    (:`PackageMissing`
      _)
    (:`PackageVersion`
      _)
    (:`NoDownload`
      _)
    (:`TravelFailure`
      _)
    (:`CheatCommands`
      _)
    (:`PendingNetGameCreateFailure`
      _)
    (:`CloudSaveFailure`
      _)
    (:`ServerTravelFailure`
      _)
    (:`ClientTravelFailure`
      _))
  (`KismetSystemLibrary.PrintString` (`|GetEnumeratorNameAsString` FailureType)))

(event `CreateSession`
  (`CreateSessionCallbackProxy.CreateSession` (`GameplayStatics.GetPlayerController` 0) 2 true
    (:`OnSuccess`
      (`KismetSystemLibrary.PrintString` "Success Create Session")
      (`GameplayStatics.OpenLevel` "TestLevel" true "Listen"))
    (:`OnFailure`
      (`KismetSystemLibrary.PrintString` "Failure Create Session"))))

(event `JoinSession`
  (bind _results (`FindSessionsCallbackProxy.FindSessions` (`GameplayStatics.GetPlayerController` 0) 1 true)
    (:`OnSuccess`
      (`KismetSystemLibrary.PrintString` "Success Find Session")
      (`JoinSessionCallbackProxy.JoinSession` (`GameplayStatics.GetPlayerController` 0) (`|GetArrayItem` _results)
        (:`OnSuccess`
          (`KismetSystemLibrary.PrintString` "Success Join Session"))
        (:`OnFailure`
          (`KismetSystemLibrary.PrintString` "Failure Join Session"))))
    (:`OnFailure`
      (`KismetSystemLibrary.PrintString` "Failure Find Session"))))

(event `SetPlayerData`
  (params (PlayerData :type "/Game/DevelopTest/BluePrints/Character/ST_PlayerData Structure"))
  (set `self.IsSavePlayerData` true)
  (set `self.PlayerData` PlayerData))

(event `MoveLevel`
  (params (LevelName :type Name))
  (`GameplayStatics.OpenLevel` LevelName true "Listen"))