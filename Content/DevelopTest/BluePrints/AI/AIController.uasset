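; AI controller for MyCharacter pawns that runs the BT_AIController behavior tree on the BB_AIController blackboard.
; Tick copies the pawn's IsAttackNotice flag into the blackboard.
; While the pawn is alive, perception updates pick out actors on other teams, write whether they are sensed to IsSearch and pass the target to the pawn through AISetEnemyInfo.
; A separate function sets IsEnableFirstAttack to true.
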(event `self.ReceiveBeginPlay`
  (`self.UseBlackboard` "/Game/DevelopTest/BluePrints/AI/BB_AIController.BB_AIController")
  (`self.RunBehaviorTree` "/Game/DevelopTest/BluePrints/AI/BT_AIController.BT_AIController"))

(event `self.ReceiveTick`
  (params (DeltaSeconds :type "Float (single-precision)"))
  (`self.SetIsAttackNotice`))

(event `self.AIPerception.OnPerceptionUpdated`
  (params (UpdatedActors :type "Array of Actor Object Reference (by ref)"))
  (`self.SetIsSerch` UpdatedActors))

(fn `InitializeBlackboardValue`
  (`BlackboardComponent.SetValueAsBool` (`AIBlueprintHelperLibrary.GetBlackboard` self) "IsEnableFirstAttack" true))

(fn `SetIsAttackNotice`
  (`BlackboardComponent.SetValueAsBool` (`AIBlueprintHelperLibrary.GetBlackboard` self) "IsAttackNotice" (`/Game/DevelopTest/BluePrints/Character/MyCharacter.IsAttackNotice` (cast `/Game/DevelopTest/BluePrints/Character/MyCharacter` (`self.K2_GetPawn`) :!pure true))))

(fn `SetIsSerch`
  (params (UpdatedActors :type "Array of Actor Object Reference"))
  (if (> (`/Game/DevelopTest/BluePrints/Character/MyCharacter.HP` (cast `/Game/DevelopTest/BluePrints/Character/MyCharacter` (`self.K2_GetPawn`) :!pure true)) 0.0)
    (for _array_element UpdatedActors
      (bind _info (`AIPerceptionComponent.GetActorsPerception` (`self.AIPerception`) _array_element))
      (bind (_target _lastsensedstimuli) (break `ActorPerceptionBlueprintInfo` _info))
      (if (!= (`/Game/DevelopTest/BluePrints/Character/MyCharacter.TeamID` (cast `/Game/DevelopTest/BluePrints/Character/MyCharacter` (`self.K2_GetPawn`) :!pure true)) (`/Game/DevelopTest/BluePrints/Character/MyCharacter.TeamID` (cast `/Game/DevelopTest/BluePrints/Character/MyCharacter` _target :!pure true)))
        (set `self.TargetActor` _target)
        (bind (_age _expirationage _strength _stimuluslocation _receiverlocation _tag _bsuccessfullysensed) (break `AIStimulus` (`|GetArrayItem` _lastsensedstimuli)))
        (`BlackboardComponent.SetValueAsBool` (`AIBlueprintHelperLibrary.GetBlackboard` self) "IsSearch" _bsuccessfullysensed)
        (`/Game/DevelopTest/BluePrints/Character/MyCharacter.AI_SetEnemyInfo` (cast `/Game/DevelopTest/BluePrints/Character/MyCharacter` (`self.K2_GetPawn`) :!pure true) _bsuccessfullysensed (`self.TargetActor`))))))

(fn `UserConstructionScript`)